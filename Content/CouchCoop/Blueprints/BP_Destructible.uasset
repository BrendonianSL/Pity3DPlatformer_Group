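; Destructible prop actor that fractures from point damage and can sink out of the world afterward.
; The construction script assigns the mesh and fits a Box collider to its bounds, blocking characters as a workaround for fracture mesh collision.
; Fracturing disables the Box, then after a delay enables Tick if ShrinkAway is set.
; Despite its name, Shrink lowers the mesh rather than scaling it, until a world-height threshold destroys the actor.
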(event OnComponentFracture(Destructible)
  (params (HitPoint :type Vector%20%28by%20ref%29 :default "0, 0, 0") (HitDirection :type Vector%20%28by%20ref%29 :default "0, 0, 0"))
  ;[1 1 1] On fracture handle collison wait 10 seconds and check if should shrink
  (Collision|SetCollisionEnabled (Variables|Default|GetBox) "NoCollision")
  (Utilities|FlowControl|Delay 1e+01)
  (if (Variables|Default|GetShrinkAway?)
    (Actor|Tick|SetActorTickEnabled true)))

(event Game|Damage|EventPointDamage
  (params (Damage :type Float%20%28single-precision%29) (DamageType :type Damage%20Type%20Object%20Reference) (HitLocation :type Vector :default "0, 0, 0") (HitNormal :type Vector :default "0, 0, 0") (HitComponent :type Primitive%20Component%20Object%20Reference) (BoneName :type Name :default "None") (ShotFromDirection :type Vector :default "0, 0, 0") (InstigatedBy :type Controller%20Object%20Reference) (DamageCauser :type Actor%20Object%20Reference) (HitInfo :type Hit%20Result%20Structure%20%28by%20ref%29))
  ;[1 0.6989 0.1622] You will want to update this actor based on the damage detection and collision methods you use within your game.
  (Class|DestructibleComponent|ApplyDamage (Variables|Default|GetDestructible) Damage HitLocation (.ImpactPoint (Collision|BreakHitResult HitInfo)) (* Damage (Variables|Default|GetImpulseStrength))))

(event EventTick
  (params (DeltaSeconds :type Float%20%28single-precision%29))
  ;[1 0.8771 0.1703] Event Tick
  (CallFunction|Shrink)
  ;;[1 1 1] Shrunk enough to destroy?
  (if (< (.Z (Math|Vector|BreakVector (Variables|Default|GetNew%20Loc))) -7e+02)
    (Actor|DestroyActor)))

(fn ConstructionScript
  (bind _destructiblemesh (Variables|Default|GetDestructibleMesh))
  (bind _box (Variables|Default|GetBox))
  (bind _returnvalue (StaticMesh|GetBounds _destructiblemesh))
  (bind (_origin _boxextent) (Math|BoxSphereBounds|BreakBoxSphereBounds _returnvalue))
  ;[1 1 1] Handle Collision to block character and work around issue with fracture mesh collision (Not sure how to disable after fracture)
  (Class|DestructibleComponent|SetDestructibleMesh (Variables|Default|GetDestructible) _destructiblemesh)
  (Transformation|SetRelativeLocation _box _origin false false)
  (Components|Box|SetBoxExtent _box _boxextent true))

(fn Shrink
  (Variables|Default|SetNew%20Loc (- (Transformation|GetWorldLocation (Variables|Default|GetDestructible)) (Math|Vector|MakeVector 0.0 0.0 (Variables|Default|GetShrinkRate))))
  (Transformation|SetWorldLocation (Variables|Default|GetDestructible) (Variables|Default|GetNew%20Loc) false false))