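; BP_Trampoline is a trampoline actor that bounces ThirdPersonCharacter players who fall into its JUMPZONE.
; On overlap, on the server or locally controlling client, it applies a movement impulse whose upward part scales with fall speed by BounceAmount, up to a cap.
; The horizontal part adds current velocity to a FacingPushRate push along the character's forward vector, and a sound plays at the jumper's location.
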(event OnComponentBeginOverlap(JUMPZONE)
  (params (OverlappedComponent :type Primitive%20Component%20Object%20Reference) (OtherActor :type Actor%20Object%20Reference) (OtherComp :type Primitive%20Component%20Object%20Reference) (OtherBodyIndex :type Integer) (bFromSweep :type Boolean) (SweepResult :type Hit%20Result%20Structure%20%28by%20ref%29))
  (bind _facingpushrate (Variables|Default|GetFacingPushRate))
  (bind _asthird_person_character (Utilities|Casting|CastToThirdPersonCharacter OtherActor))
  (Variables|Default|SetJumper _asthird_person_character)
  (if (or (Pawn|IsLocallyControlled _asthird_person_character) (Ability|HasAuthority))
    (if (> (.Z (Math|Vector|BreakVector (* (Variables|/Script/Engine.MovementComponent|GetVelocity (Variables|/Script/Engine.Character|GetCharacterMovement (Variables|Default|GetJumper))) -1.0))) 0.0)
      (Physics|AddImpulse (Variables|/Script/Engine.Character|GetCharacterMovement (Variables|Default|GetJumper)) (Math|Vector|MakeVector (+ (.X (Math|Vector|BreakVector (Variables|/Script/Engine.MovementComponent|GetVelocity (Variables|/Script/Engine.Character|GetCharacterMovement (Variables|Default|GetJumper))))) (* (.x (Transformation|GetActorForwardVector (Variables|Default|GetJumper))) _facingpushrate)) (+ (* (.y (Transformation|GetActorForwardVector (Variables|Default|GetJumper))) _facingpushrate) (.Y (Math|Vector|BreakVector (Variables|/Script/Engine.MovementComponent|GetVelocity (Variables|/Script/Engine.Character|GetCharacterMovement (Variables|Default|GetJumper)))))) (Math|Float|Clamp(Float) (* (.Z (Math|Vector|BreakVector (* (Variables|/Script/Engine.MovementComponent|GetVelocity (Variables|/Script/Engine.Character|GetCharacterMovement (Variables|Default|GetJumper))) -1.0))) (Variables|Default|GetBounceAmount)) 0.0 1.5e+05)) false)
      (Audio|PlaySoundatLocation "/Engine/VREditor/Sounds/UI/Laser_Push.Laser_Push" (Transformation|GetActorLocation (Variables|Default|GetJumper)) "0, 0, 0" 1.0 1.0 0.0 0 0 0))))

(fn ConstructionScript)