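; Child bounce pad Blueprint that plays a visual impact reaction through its material when hit or when something enters its jump zone.
; At BeginPlay it creates a dynamic material instance on its static mesh.
; Both events set the material's position to the impact point and restart the Bounce timeline, which drives an impact vector along the normal.
; Both read the overlap's sweep result, leaving the hit event's own result unused.
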(event OnComponentHit(StaticMeshComponent)
  (params (HitComponent :type Primitive%20Component%20Object%20Reference) (OtherActor :type Actor%20Object%20Reference) (OtherComp :type Primitive%20Component%20Object%20Reference) (NormalImpulse :type Vector :default "0, 0, 0") (Hit :type Hit%20Result%20Structure%20%28by%20ref%29))
  (bind _material (Variables|Default|GetMaterial))
  (Rendering|Material|SetVectorParameterValue _material "pos" (Math|Conversions|ToLinearColor(Vector) (.ImpactPoint (Collision|BreakHitResult (stale OnComponentBeginOverlap(JUMPZONE) SweepResult)))) :!class /Script/Engine.MaterialInstanceDynamic)
  (bind _newtrack_0 (Timeline|Bounce PlayFromStart)
    (:Update
      (Rendering|Material|SetVectorParameterValue _material "impact" (Math|Conversions|ToLinearColor(Vector) (* (.ImpactNormal (Collision|BreakHitResult (stale OnComponentBeginOverlap(JUMPZONE) SweepResult))) (* _newtrack_0 25.0))) :!class /Script/Engine.MaterialInstanceDynamic))))

(event OnComponentBeginOverlap(JUMPZONE)
  (params (OverlappedComponent :type Primitive%20Component%20Object%20Reference) (OtherActor :type Actor%20Object%20Reference) (OtherComp :type Primitive%20Component%20Object%20Reference) (OtherBodyIndex :type Integer) (bFromSweep :type Boolean) (SweepResult :type Hit%20Result%20Structure%20%28by%20ref%29))
  (bind (_bblockinghit _binitialoverlap _time _distance _location _impactpoint _normal _impactnormal) (Collision|BreakHitResult SweepResult))
  (bind _material (Variables|Default|GetMaterial))
  (Rendering|Material|SetVectorParameterValue _material "pos" (Math|Conversions|ToLinearColor(Vector) _impactpoint) :!class /Script/Engine.MaterialInstanceDynamic)
  (bind _newtrack_0 (Timeline|Bounce PlayFromStart)
    (:Update
      (Rendering|Material|SetVectorParameterValue _material "impact" (Math|Conversions|ToLinearColor(Vector) (* _impactnormal (* _newtrack_0 25.0))) :!class /Script/Engine.MaterialInstanceDynamic))))

(event EventBeginPlay
  (bind _returnvalue (Rendering|Material|CreateDynamicMaterialInstance (Variables|Default|GetStaticMeshComponent) 0 0 "None" :!class /Script/Engine.PrimitiveComponent))
  (Variables|Default|SetMaterial _returnvalue))

(fn ConstructionScript
  (|CallParentFunction))