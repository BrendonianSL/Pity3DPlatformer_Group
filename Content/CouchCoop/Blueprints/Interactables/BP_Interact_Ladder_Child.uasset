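; Climbable ladder interactable for couch co-op, a child Blueprint that lets a player move vertically along it.
; Interact stores the character, enables ladder input for that player's controller by index and switches movement to Flying, so MoveForward moves the stored character along its up vector.
; When a ThirdPersonCharacter stops overlapping the box, the ladder disables that player's input and restores Walking.
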(event OnComponentEndOverlap(Box)
  (params (OverlappedComponent :type Primitive%20Component%20Object%20Reference) (OtherActor :type Actor%20Object%20Reference) (OtherComp :type Primitive%20Component%20Object%20Reference) (OtherBodyIndex :type Integer))
  (bind _asthird_person_character (Utilities|Casting|CastToThirdPersonCharacter OtherActor))
  (Input|DisableInput (Class|GameplayStatics|GetPlayerControllerfromID (Variables|/Game/CouchCoop/Blueprints/ThirdPersonCharacter.ThirdPersonCharacter_C|GetIndex _asthird_person_character)))
  (Pawn|Components|CharacterMovement|SetMovementMode (Variables|/Script/Engine.Character|GetCharacterMovement _asthird_person_character) "MOVE_Walking" 0))

(event EventBeginPlay
  (|CallParentFunction) ; This node is disabled and will not be called.\nDrag off pins to build functionality.
)

(event EventInteract
  (params (Character :type Third%20Person%20Character%20Object%20Reference))
  (bind _output_get (Variables|Default|SetCharacter Character))
  (Input|EnableInput (Class|GameplayStatics|GetPlayerControllerfromID (Variables|/Game/CouchCoop/Blueprints/ThirdPersonCharacter.ThirdPersonCharacter_C|GetIndex _output_get)))
  (Pawn|Components|CharacterMovement|SetMovementMode (Variables|/Script/Engine.Character|GetCharacterMovement _output_get) "MOVE_Flying" 0))

(event EventTick
  (params (DeltaSeconds :type Float%20%28single-precision%29))
  (|CallParentFunction DeltaSeconds) ; This node is disabled and will not be called.\nDrag off pins to build functionality.
)

(event Input|AxisEvents|InputAxisMoveForward
  (params (AxisValue :type Float%20%28single-precision%29))
  (bind _character (Variables|Default|GetCharacter))
  (Pawn|Input|AddMovementInput _character (Transformation|GetActorUpVector _character) AxisValue false))

(fn ConstructionScript
  (|CallParentFunction))